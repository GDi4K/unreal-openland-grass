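; BP_OpenLand_Grass_Tools is a helper Blueprint that exposes setter functions for tuning OpenLand grass material parameters.
; Each function writes one parameter in the MPC_OpenLand_Grass Material Parameter Collection, covering wind, RVT distance blending and grass hiding, Z offset, and variation tiling.
; AddDirectionalWind turns a yaw angle and intensity into a vector and overwrites the Directional Wind parameter rather than accumulating it.
; BeginPlay and Tick are empty, so changes occur only when these functions are called.
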(event EventBeginPlay)

(event EventTick
  (params (DeltaSeconds :type Float%20%28single-precision%29)))

(fn AddDirectionalWind
  (params (Direction%20Angle :type Integer) (Intensity :type Float%20%28single-precision%29))
  (Rendering|Material|SetVectorParameterValue "/Game/OpenLandGrass/Materials/MPC_OpenLand_Grass.MPC_OpenLand_Grass" "Directional Wind" (Math|Conversions|ToLinearColor(Vector) (Math|Vector|RotateVector (* "1.000000, 0, 0" Intensity) (Math|Rotator|MakeRotator 0.0 0.0 (Math|Conversions|ToFloat(Integer) Direction%20Angle)))) :!class /Script/Engine.KismetMaterialLibrary))

(fn SetWindIntensity
  (params (Value :type Float%20%28single-precision%29))
  (Rendering|Material|SetScalarParameterValue "/Game/OpenLandGrass/Materials/MPC_OpenLand_Grass.MPC_OpenLand_Grass" "Wind Intensity Multipliar" Value :!class /Script/Engine.KismetMaterialLibrary))

(fn SetWindModulationFactor
  (params (Value :type Float%20%28single-precision%29))
  (Rendering|Material|SetScalarParameterValue "/Game/OpenLandGrass/Materials/MPC_OpenLand_Grass.MPC_OpenLand_Grass" "Wind Modulation Factor" Value :!class /Script/Engine.KismetMaterialLibrary))

(fn SetWindPlaneTilingFactor
  (params (Value :type Float%20%28single-precision%29))
  (Rendering|Material|SetScalarParameterValue "/Game/OpenLandGrass/Materials/MPC_OpenLand_Grass.MPC_OpenLand_Grass" "Wind Plane Tiling Factor" Value :!class /Script/Engine.KismetMaterialLibrary))

(fn SetRVTDistanceBlendingIntensity
  (params (Value :type Float%20%28single-precision%29))
  (Rendering|Material|SetScalarParameterValue "/Game/OpenLandGrass/Materials/MPC_OpenLand_Grass.MPC_OpenLand_Grass" "RVT Distance Blending Intensity" Value :!class /Script/Engine.KismetMaterialLibrary))

(fn SetRVTDistanceBlendingThreshold
  (params (Value :type Float%20%28single-precision%29))
  (Rendering|Material|SetScalarParameterValue "/Game/OpenLandGrass/Materials/MPC_OpenLand_Grass.MPC_OpenLand_Grass" "RVT Distance Blending Threshold" Value :!class /Script/Engine.KismetMaterialLibrary))

(fn SetRVTDistanceBlendingFalloff
  (params (Value :type Float%20%28single-precision%29))
  (Rendering|Material|SetScalarParameterValue "/Game/OpenLandGrass/Materials/MPC_OpenLand_Grass.MPC_OpenLand_Grass" "RVT Distance Blending Falloff" Value :!class /Script/Engine.KismetMaterialLibrary))

(fn SetZOffsetDistanceThreshold
  (params (Value :type Float%20%28single-precision%29))
  (Rendering|Material|SetScalarParameterValue "/Game/OpenLandGrass/Materials/MPC_OpenLand_Grass.MPC_OpenLand_Grass" "Z Offset Distance Threshold" Value :!class /Script/Engine.KismetMaterialLibrary))

(fn SetZOffsetDistanceFalloff
  (params (Value :type Float%20%28single-precision%29))
  (Rendering|Material|SetScalarParameterValue "/Game/OpenLandGrass/Materials/MPC_OpenLand_Grass.MPC_OpenLand_Grass" "Z Offset Distance Falloff" Value :!class /Script/Engine.KismetMaterialLibrary))

(fn SetZOffsetMultiplier
  (params (Value :type Float%20%28single-precision%29))
  (Rendering|Material|SetScalarParameterValue "/Game/OpenLandGrass/Materials/MPC_OpenLand_Grass.MPC_OpenLand_Grass" "Z Offset Multiplier" Value :!class /Script/Engine.KismetMaterialLibrary))

(fn SetVariationTilingFactor
  (params (Value :type Float%20%28single-precision%29))
  (Rendering|Material|SetScalarParameterValue "/Game/OpenLandGrass/Materials/MPC_OpenLand_Grass.MPC_OpenLand_Grass" "Variation Tiling Factor" Value :!class /Script/Engine.KismetMaterialLibrary))

(fn SetRVTHideGrassIntensity
  (params (Value :type Float%20%28single-precision%29))
  (Rendering|Material|SetScalarParameterValue "/Game/OpenLandGrass/Materials/MPC_OpenLand_Grass.MPC_OpenLand_Grass" "RVT Hide Grass Intensity" Value :!class /Script/Engine.KismetMaterialLibrary))