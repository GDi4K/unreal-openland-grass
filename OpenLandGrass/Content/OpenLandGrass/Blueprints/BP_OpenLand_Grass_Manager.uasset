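; OpenLand grass manager actor that applies shared grass settings through the OpenLandGrassTools function library.
; Main runs from both the construction script and BeginPlay, so settings take effect in the editor and at game start.
; It pushes the actor's variables in grouped steps: directional wind, RVT distance blending and grass hiding, Z-offset distance blending, and variation tiling.
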(event EventBeginPlay
  (CallFunction|Main))

(event Collision|EventActorBeginOverlap
  (params (OtherActor :type Actor%20Object%20Reference)))

(event EventTick
  (params (DeltaSeconds :type Float%20%28single-precision%29)))

(fn ConstructionScript
  (CallFunction|Main))

(fn Main
  (Utilities|FlowControl|Sequence
    (:then_0
      ;[1 1 1] Wind Controls
      (Default|AddDirectionalWind (Variables|Default|GetOpenLandGrassTools) (Variables|DirectionalWind|GetWind%20Direction) (Variables|DirectionalWind|GetDirectional%20Wind%20Intensity))
      (Default|SetWindIntensity (Variables|Default|GetOpenLandGrassTools) (Variables|Wind|GetWind%20Intensity%20Multipliar))
      (Default|SetWindModulationFactor (Variables|Default|GetOpenLandGrassTools) (Variables|Wind|GetWind%20Modulation%20Factor))
      (Default|SetWindPlaneTilingFactor (Variables|Default|GetOpenLandGrassTools) (Variables|Wind|GetWind%20Plane%20Tiling%20Factor)))
    (:then_1
      ;[1 1 1] RVT Distance Blend
      (Default|SetRVTDistanceBlendingIntensity (Variables|Default|GetOpenLandGrassTools) (Variables|RVTDistanceBlending|GetRVT%20Distance%20Blending%20Intensity))
      (Default|SetRVTDistanceBlendingThreshold (Variables|Default|GetOpenLandGrassTools) (Variables|RVTDistanceBlending|GetRVT%20Distance%20Threshold))
      (Default|SetRVTDistanceBlendingFalloff (Variables|Default|GetOpenLandGrassTools) (Variables|RVTDistanceBlending|GetRVT%20Distance%20Falloff)))
    (:then_2
      ;[1 1 1] Other RVT Parameters
      (Default|SetRVTHideGrassIntensity (Variables|Default|GetOpenLandGrassTools) (Variables|RVTMisc|GetRVT%20Hide%20Grass%20Intensity)))
    (:then_3
      ;[1 1 1] Z Offset Distance Blending
      (Default|SetZOffsetMultiplier (Variables|Default|GetOpenLandGrassTools) (Variables|ZOffsetDistanceBlending|GetZ%20Offset%20Distance%20Multiplier))
      (Default|SetZOffsetDistanceThreshold (Variables|Default|GetOpenLandGrassTools) (Variables|ZOffsetDistanceBlending|GetZ%20Offset%20Distance%20Threshold))
      (Default|SetZOffsetDistanceFalloff (Variables|Default|GetOpenLandGrassTools) (Variables|ZOffsetDistanceBlending|GetZ%20Offset%20Distance%20Falloff)))
    (:then_4
      ;[1 1 1] Variations
      (Default|SetVariationTilingFactor (Variables|Default|GetOpenLandGrassTools) (Variables|Variations|GetVariation%20Tiling%20Factor)))))